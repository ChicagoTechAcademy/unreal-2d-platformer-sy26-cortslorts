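; BP_Slime is a PaperZD-animated slime enemy that dies when the player character overlaps its StompBox.
; The overlap disables capsule and stomp collision, then plays the Death sequence as an animation override.
; A delay driven by that override's return value precedes destroying the actor.
; Tick is empty, and a forward movement input node is present but never runs.
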(event OnComponentBeginOverlap(StompBox)
  (params (OverlappedComponent :type Primitive%20Component%20Object%20Reference) (OtherActor :type Actor%20Object%20Reference) (OtherComp :type Primitive%20Component%20Object%20Reference) (OtherBodyIndex :type Integer) (bFromSweep :type Boolean) (SweepResult :type Hit%20Result%20Structure%20%28by%20ref%29))
  (Utilities|Casting|CastToBP_PlayerCharacter OtherActor)
  (Collision|SetCollisionEnabled (Variables|Default|GetCapsuleComponent) "NoCollision")
  (Collision|SetCollisionEnabled (Variables|Default|GetStompBox) "NoCollision")
  (bind _animationlength (Class|PaperZDAnimInstance|PlayAnimationOverride (Variables|/Script/PaperZD.PaperZDAnimationComponent|GetAnimInstance (Variables|Default|GetPaperZDAnimation)) "/Game/BluePrints/Enimies/Slime/AnimSequences/Death.Death" "DeathAnim" 1.0 0.0))
  (Utilities|FlowControl|Delay _animationlength)
  (Actor|DestroyActor))

(event EventBeginPlay)

(event Collision|EventActorBeginOverlap
  (params (OtherActor :type Actor%20Object%20Reference)))

(event EventTick
  (params (DeltaSeconds :type Float%20%28single-precision%29)))

(fn ConstructionScript
  (|CallParentFunction))